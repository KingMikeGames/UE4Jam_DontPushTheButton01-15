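; RoadActor is an actor that builds a road mesh along its spline.
; UpdateRoad steps along the spline at Spacing intervals, adding a collision-enabled spline mesh per step with a plane mesh and grimy concrete material.
; Each segment takes world-space start and end points and direction tangents scaled by TangentScale from the spline, using manual attachment.
; The construction script and events are empty, so nothing here calls UpdateRoad.
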(event EventBeginPlay)

(event EventActorBeginOverlap
  (params (OtherActor :type Actor%20Object%20Reference)))

(event EventTick
  (params (DeltaSeconds :type Float%20%28single-precision%29)))

(fn ConstructionScript)

(fn UpdateRoad
  (bind _spline (Variables|Default|GetSpline))
  (bind _tangentscale (Variables|Default|GetTangentScale))
  (bind _spacing (Variables|Default|GetSpacing))
  (for _index (range 0 (.ReturnValue (Math|Float|Division(WholeandRemainder) (Spline|GetSplineLength (Variables|Default|GetSpline)) _spacing)))
    (bind _returnvalue (AddComponent|AddSplineMeshComponent true))
    (Collision|SetCollisionEnabled _returnvalue "QueryAndPhysics")
    (SplineMesh|SetStartandEnd _returnvalue (Spline|GetLocationatDistanceAlongSpline _spline (* _index _spacing) "World") (* (Spline|GetDirectionatDistanceAlongSpline _spline (* _index _spacing) "World") _tangentscale) (Spline|GetLocationatDistanceAlongSpline _spline (+ (* _index _spacing) (Variables|Default|GetSpacing)) "World") (* (Spline|GetDirectionatDistanceAlongSpline _spline (+ (* _index _spacing) (Variables|Default|GetSpacing)) "World") _tangentscale) :!class /Script/Engine.SplineMeshComponent)
    (Components|StaticMesh|SetStaticMesh _returnvalue "/Game/StarterContent/Shapes/Shape_Plane.Shape_Plane")
    (Rendering|Material|SetMaterial _returnvalue 0 "/Game/StarterContent/Materials/M_Concrete_Grime.M_Concrete_Grime")))