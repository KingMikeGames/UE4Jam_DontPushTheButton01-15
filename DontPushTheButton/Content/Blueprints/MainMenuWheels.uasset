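; Main menu wheel actor that displays the player's equipped wheel style on its Cylinder mesh.
; On BeginPlay it waits briefly, refreshes, then registers itself in the game mode's MainMenuWheels list.
; Refresh sets the material by indexing the game instance's WheelMaterials array with EquippedWheels.
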(event Custom|Refresh
  (bind _returnvalue (Game|GetGameInstance))
  (bind _asthe_game_instance (Utilities|Casting|CastToTheGameInstance _returnvalue))
  (Rendering|Material|SetMaterial (Variables|Default|GetCylinder) 0 (Utilities|Array|Get(acopy) (Variables|/Game/GameInstance/TheGameInstance.TheGameInstance_C|GetWheelMaterials _asthe_game_instance) (Variables|/Game/GameInstance/TheGameInstance.TheGameInstance_C|GetEquippedWheels _asthe_game_instance))))

(event EventBeginPlay
  (Utilities|FlowControl|Delay 0.2)
  (CallFunction|Refresh)
  (Utilities|Array|AddUnique (Variables|/Game/GameMode/TheGameMode.TheGameMode_C|GetMainMenuWheels (.AsThe%20Game%20Mode (Utilities|Casting|CastToTheGameMode (Game|GetGameMode)))) self))

(event EventActorBeginOverlap
  (params (OtherActor :type Actor%20Object%20Reference)))

(event EventTick
  (params (DeltaSeconds :type Float%20%28single-precision%29)))

(fn ConstructionScript)