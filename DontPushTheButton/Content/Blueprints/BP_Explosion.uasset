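; BP_Explosion is an actor that travels along the road's spline; the graph contains only this movement, with no effect or damage logic.
; On BeginPlay it takes the first RoadActor found, stores its Spline and places itself at the start.
; Each Tick adds Speed to the distance without delta-time scaling, then moves to that world-space spline point with the Y coordinate multiplied by a constant.
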(event EventActorBeginOverlap
  (params (OtherActor :type Actor%20Object%20Reference)))

(event EventTick
  (params (DeltaSeconds :type Float%20%28single-precision%29))
  (bind _output_get (Variables|Default|SetDistanceAlongSpline (+ (Variables|Default|GetDistanceAlongSpline) (Variables|Default|GetSpeed))))
  (Transformation|SetActorLocation (Math|Vector|MakeVector (.X (Math|Vector|BreakVector (Spline|GetLocationatDistanceAlongSpline (Variables|Default|GetSpline) _output_get "World"))) (* (.Y (Math|Vector|BreakVector (Spline|GetLocationatDistanceAlongSpline (Variables|Default|GetSpline) _output_get "World"))) 2e+01) (.Z (Math|Vector|BreakVector (Spline|GetLocationatDistanceAlongSpline (Variables|Default|GetSpline) _output_get "World")))) false false))

(event EventBeginPlay
  (bind _outactors (Actor|GetAllActorsOfClass "/Game/Blueprints/RoadActor.RoadActor_C"))
  (Variables|Default|SetSpline (Variables|/Game/Blueprints/RoadActor.RoadActor_C|GetSpline (Utilities|Array|Get(acopy) _outactors)))
  (Variables|Default|SetDistanceAlongSpline 0.0)
  (Transformation|SetActorLocation (Math|Vector|MakeVector (.X (Math|Vector|BreakVector (Spline|GetLocationatDistanceAlongSpline (Variables|Default|GetSpline) (stale EventTick _output_get) "World"))) (* (.Y (Math|Vector|BreakVector (Spline|GetLocationatDistanceAlongSpline (Variables|Default|GetSpline) (stale EventTick _output_get) "World"))) 2e+01) (.Z (Math|Vector|BreakVector (Spline|GetLocationatDistanceAlongSpline (Variables|Default|GetSpline) (stale EventTick _output_get) "World")))) false false))

(fn ConstructionScript)