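; Endless procedural track generator that lays road spline meshes along a spline at BeginPlay, then extends it on a looping timer.
; Each tick of the timer adds a point ahead of the last one with random offset and randomised bank, width and thickness defaults.
; UpdateRoadDataArray syncs per-point data to the point count, which BuildTrackElement uses for each segment's roll and scale.
; The last mesh is destroyed and rebuilt alongside the new segment.
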(event Custom|CustomEvent_0
  (bind _returnvalue (Math|Random|RandomUnitVector))
  (bind _splinemesh (Variables|Default|GetsplineMesh))
  (bind _spline (Variables|Default|GetSpline))
  (Components|DestroyComponent (Utilities|Array|Get(acopy) _splinemesh (Utilities|Array|LastIndex _splinemesh)))
  (Variables|Default|SetRoadMeshDefaults (Utilities|Struct|MakeRoadData false false (Math|Random|RandomFloatinRange -0.4 0.4) (Math|Random|RandomFloatinRange 0.4 2.0) (Math|Random|RandomFloatinRange 1.0 4.0)))
  (Spline|AddSplinePoint (Variables|Default|GetSpline) (+ (+ (* (Math|Vector|Normalize (Math|Vector|MakeVector (.x (Class|SplineComponent|GetDirectionatSplinePoint _spline (- (Variables|Default|GetNumberOfSplinePoints) 1) "World")) (.y (Class|SplineComponent|GetDirectionatSplinePoint _spline (- (Variables|Default|GetNumberOfSplinePoints) 1) "World")) 0.0)) 5e+03) (Spline|GetLocationatSplinePoint _spline (- (Variables|Default|GetNumberOfSplinePoints) 1) "Local")) (Math|Vector|MakeVector (* (.x _returnvalue) 2.5e+03) (* (.y _returnvalue) 4e+03) (* (.z _returnvalue) 1e+03))) "Local")
  (Variables|Default|SetNumberOfSplinePoints (Spline|GetNumberOfSplinePoints (Variables|Default|GetSpline)))
  (CallFunction|UpdateRoadDataArray)
  (for _index (range (- (Variables|Default|GetNumberOfSplinePoints) 3) (- (Variables|Default|GetNumberOfSplinePoints) 1))
    (CallFunction|BuildTrackElement _index (Variables|Default|GetRoadMesh))))

(event EventBeginPlay
  (Utilities|FlowControl|Sequence
    (:then_0
      (Variables|Default|SetNumberOfSplinePoints (Spline|GetNumberOfSplinePoints (Variables|Default|GetSpline))))
    (:then_1
      (CallFunction|UpdateRoadDataArray))
    (:then_2
      (for _index (range 0 (- (Variables|Default|GetNumberOfSplinePoints) 1))
        (CallFunction|BuildTrackElement _index (Variables|Default|GetRoadMesh))))
    (:then_3
      (Utilities|Time|SetTimerbyEvent (delegate Custom|CustomEvent_0) 2.0 true))))

(event EventTick
  (params (DeltaSeconds :type Float%20%28single-precision%29)))

(fn ConstructionScript)

(fn BuildTrackElement
  (params (LoopIndex :type Integer) (TrackElementMesh :type Static%20Mesh%20Object%20Reference))
  (if (not (== LoopIndex (- (Variables|Default|GetNumberOfSplinePoints) 1)))
    (LocalVariables|SetLocal_CurrentLoopIndex LoopIndex)
    (LocalVariables|SetLocal_NextLoopIndex (Math|Integer|%(Integer) (+ LoopIndex 1) (Variables|Default|GetNumberOfSplinePoints)))
    (LocalVariables|SetLocal_TrackElementMesh TrackElementMesh)
    (Utilities|FlowControl|Sequence
      (:then_0
        (LocalVariables|SetLocal_StartLocation (.Location (Spline|GetLocationandTangentatSplinePoint (Variables|Default|GetSpline) (LocalVariables|GetLocal_CurrentLoopIndex) "Local")))
        (LocalVariables|SetLocal_StartTangent (.Tangent (Spline|GetLocationandTangentatSplinePoint (Variables|Default|GetSpline) (LocalVariables|GetLocal_CurrentLoopIndex) "Local")))
        (LocalVariables|SetLocal_EndLocation (.Location (Spline|GetLocationandTangentatSplinePoint (Variables|Default|GetSpline) (LocalVariables|GetLocal_NextLoopIndex) "Local")))
        (LocalVariables|SetLocal_EndTangent (.Tangent (Spline|GetLocationandTangentatSplinePoint (Variables|Default|GetSpline) (LocalVariables|GetLocal_NextLoopIndex) "Local"))))
      (:then_1
        (bind _returnvalue (AddComponent|AddSplineMeshComponent false))
        (LocalVariables|SetLocal_CurrentSplineMesh _returnvalue)
        (Collision|SetCollisionEnabled _returnvalue "QueryAndPhysics")
        (SplineMesh|SetStartandEnd (LocalVariables|GetLocal_CurrentSplineMesh) (LocalVariables|GetLocal_StartLocation) (LocalVariables|GetLocal_StartTangent) (LocalVariables|GetLocal_EndLocation) (LocalVariables|GetLocal_EndTangent) :!class /Script/Engine.SplineMeshComponent)
        (LocalVariables|SetLocal_StartRoll (.trackbank (Utilities|Array|Get(acopy) (Variables|Default|GetRoadDataArray) (LocalVariables|GetLocal_CurrentLoopIndex))))
        (LocalVariables|SetLocal_StartScale (Math|Vector2D|MakeVector2D (.trackwidth (Utilities|Array|Get(acopy) (Variables|Default|GetRoadDataArray) (LocalVariables|GetLocal_CurrentLoopIndex))) (.trackthickness (Utilities|Array|Get(acopy) (Variables|Default|GetRoadDataArray) (LocalVariables|GetLocal_CurrentLoopIndex)))))
        (LocalVariables|SetLocal_EndRoll (.trackbank (Utilities|Array|Get(acopy) (Variables|Default|GetRoadDataArray) (LocalVariables|GetLocal_NextLoopIndex))))
        (LocalVariables|SetLocal_EndScale (Math|Vector2D|MakeVector2D (.trackwidth (Utilities|Array|Get(acopy) (Variables|Default|GetRoadDataArray) (LocalVariables|GetLocal_NextLoopIndex))) (.trackthickness (Utilities|Array|Get(acopy) (Variables|Default|GetRoadDataArray) (LocalVariables|GetLocal_NextLoopIndex)))))
        (Class|SplineMeshComponent|SetStartRoll (LocalVariables|GetLocal_CurrentSplineMesh) (LocalVariables|GetLocal_StartRoll))
        (Class|SplineMeshComponent|SetEndRoll (LocalVariables|GetLocal_CurrentSplineMesh) (LocalVariables|GetLocal_EndRoll))
        (SplineMesh|SetStartScale (LocalVariables|GetLocal_CurrentSplineMesh) (LocalVariables|GetLocal_StartScale) :!class /Script/Engine.SplineMeshComponent)
        (SplineMesh|SetEndScale (LocalVariables|GetLocal_CurrentSplineMesh) (LocalVariables|GetLocal_EndScale) :!class /Script/Engine.SplineMeshComponent)
        (Components|StaticMesh|SetStaticMesh (LocalVariables|GetLocal_CurrentSplineMesh) (LocalVariables|GetLocal_TrackElementMesh))
        (Utilities|Array|Add (Variables|Default|GetsplineMesh) (LocalVariables|GetLocal_CurrentSplineMesh))))))

(fn UpdateRoadDataArray
  (bind _roaddataarray (Variables|Default|GetRoadDataArray))
  (Math|Integer|CompareInt (Utilities|Array|Length (Variables|Default|GetRoadDataArray)) (Variables|Default|GetNumberOfSplinePoints) :!label _label
    (:>
      (Utilities|Array|RemoveIndex _roaddataarray (Utilities|Array|LastIndex _roaddataarray))
      (goto _label))
    (:<
      (Utilities|Array|Add _roaddataarray (Variables|Default|GetRoadMeshDefaults))
      (goto _label))))

(fn NewFunction0)