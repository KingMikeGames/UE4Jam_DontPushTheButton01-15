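; Display actor that shows the player's equipped trailer in the main menu.
; On BeginPlay it waits briefly, refreshes its static mesh, then registers itself with TheGameMode as MainMenuTrailer.
; Refresh sets the mesh from the game instance's Trailers array at the EquippedTrailer index.
; The stored game mode reference lets other code call Refresh on it.
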(event Custom|Refresh
  (bind _returnvalue (Game|GetGameInstance))
  (bind _asthe_game_instance (Utilities|Casting|CastToTheGameInstance _returnvalue))
  (Components|StaticMesh|SetStaticMesh (Variables|Debug|GetStaticMeshComponent) (.staticmesh (Utilities|Array|Get(acopy) (Variables|/Game/GameInstance/TheGameInstance.TheGameInstance_C|GetTrailers _asthe_game_instance) (Variables|/Game/GameInstance/TheGameInstance.TheGameInstance_C|GetEquippedTrailer _asthe_game_instance)))))

(event EventBeginPlay
  (Utilities|FlowControl|Delay 0.2)
  (CallFunction|Refresh)
  (Variables|/Game/GameMode/TheGameMode.TheGameMode_C|SetMainMenuTrailer (.AsThe%20Game%20Mode (Utilities|Casting|CastToTheGameMode (Game|GetGameMode))) self))

(event EventActorBeginOverlap
  (params (OtherActor :type Actor%20Object%20Reference)))

(event EventTick
  (params (DeltaSeconds :type Float%20%28single-precision%29)))

(fn ConstructionScript)